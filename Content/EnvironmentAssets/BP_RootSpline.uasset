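; Environment Blueprint that builds a tapering root from spline mesh segments along RootSpline.
; The Construction Script loops over the spline points, adding a SplineMeshComponent fitted to each point and the next using local locations and tangents.
; Cross-section scale starts from SplineWidth times SegmentScale and shrinks by a fixed step based on point count, each segment's end scale carrying into the next segment's start.
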(event EventBeginPlay)

(event Collision|EventActorBeginOverlap
  (params (OtherActor :type Actor%20Object%20Reference)))

(event EventTick
  (params (DeltaSeconds :type Float%20%28single-precision%29)))

(fn ConstructionScript
  (bind _rootspline (Variables|Default|GetRootSpline))
  (bind _returnvalue (Spline|GetNumberOfSplinePoints _rootspline))
  (Variables|Default|SetSegmentScale (* (Variables|Default|GetSplineWidth) (Variables|Default|GetSegmentScale)))
  (for _index (range 0 _returnvalue)
    (bind _returnvalue_2 (AddComponent|AddSplineMeshComponent false))
    (SplineMesh|SetStartandEnd _returnvalue_2 (.Location (Spline|GetLocationandTangentatSplinePoint _rootspline _index "Local")) (.Tangent (Spline|GetLocationandTangentatSplinePoint _rootspline _index "Local")) (.Location (Spline|GetLocationandTangentatSplinePoint _rootspline (+ _index 1) "Local")) (.Tangent (Spline|GetLocationandTangentatSplinePoint _rootspline (+ _index 1) "Local")) true :!class /Script/Engine.SplineMeshComponent)
    (SplineMesh|SetStartScale _returnvalue_2 (Math|Vector2D|MakeVector2D (Variables|Default|GetSegmentScale) (Variables|Default|GetSegmentScale)) true :!class /Script/Engine.SplineMeshComponent)
    (bind _output_get (Variables|Default|SetSegmentScale (- (Variables|Default|GetSegmentScale) (/ (Variables|Default|GetSplineWidth) (- (Math|Conversions|ToFloat(Integer) _returnvalue) 0.5)))))
    (SplineMesh|SetEndScale _returnvalue_2 (Math|Vector2D|MakeVector2D _output_get _output_get) true :!class /Script/Engine.SplineMeshComponent)))
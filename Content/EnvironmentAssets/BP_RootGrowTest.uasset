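; Clickable root segment that previews as a ghost on hover and grows on click, within BP_SecondPhase's click limit.
; Construction script sets mesh and animation from RootStylePicker.
; BeginPlay matches overlapping actor names against five nutrients to set WhereRootConnects.
; Growing plays the animation, removes the click target, increments the matching resource's touched count, and can reveal RootChildren as clickable after a delay, chaining growth.
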(event OnClicked(Cube)
  (params (TouchedComponent :type Primitive%20Component%20Object%20Reference) (ButtonPressed :type Key%20Structure :default "None"))
  (bind _returnvalue (Game|GetPlayerController 0))
  (bind _sk_root02_wigglyanim2 (Variables|Default|GetSK_Root02_WigglyAnim2))
  (bind _sk_root02_wigglyanim2_2 (Variables|Default|GetSK_Root02_WigglyAnim2))
  (Variables|/Script/Engine.PlayerController|SetbEnableClickEvents _returnvalue false)
  (Variables|/Script/Engine.PlayerController|SetbEnableMouseOverEvents _returnvalue false)
  (bind _returnvalue_2 (Actor|GetActorOfClass "/Game/ThirdPerson/Blueprints/BP_SecondPhase.BP_SecondPhase_C"))
  (if (Variables|Default|GetIsClickable)
    (if (not (>= (Variables|/Game/ThirdPerson/Blueprints/BP_SecondPhase.BP_SecondPhase_C|GetRootClicksCurrent _returnvalue_2) (Variables|/Game/ThirdPerson/Blueprints/BP_SecondPhase.BP_SecondPhase_C|GetRootClicksTotal _returnvalue_2)))
      (Rendering|Material|SetMaterial _sk_root02_wigglyanim2_2 1 "/Game/EnvironmentAssets/materials/M_TreeRoots.M_TreeRoots")
      (Rendering|Material|SetMaterial _sk_root02_wigglyanim2_2 0 "/Game/EnvironmentAssets/materials/M_MaskedMASTER.M_MaskedMASTER")
      (switch int (Variables|Default|GetRootStylePicker)
        (:Default
          (Components|Animation|PlayAnimation _sk_root02_wigglyanim2 "/Game/EnvironmentAssets/models/SK_Root02_WigglyAnim2.SK_Root02_WigglyAnim2_Animation" false :!label _label))
        (:0
          (goto _label))
        (:1
          (Components|Animation|PlayAnimation _sk_root02_wigglyanim2 "/Game/EnvironmentAssets/models/SK_Root03_ShortAnim.SK_Root03_ShortAnim_Animation" false))
        (:2
          (Components|Animation|PlayAnimation _sk_root02_wigglyanim2 "/Game/EnvironmentAssets/models/SK_Root04_LongAnim.SK_Root04_LongAnim_Animation" false)))
      (Components|DestroyComponent (Variables|Default|GetCube))
      (bind _returnvalue_3 (Actor|GetActorOfClass "/Game/ThirdPerson/Blueprints/BP_SecondPhase.BP_SecondPhase_C"))
      (bind _output_get (Variables|/Game/ThirdPerson/Blueprints/BP_SecondPhase.BP_SecondPhase_C|SetRootClicksCurrent _returnvalue_3 (+ (Variables|/Game/ThirdPerson/Blueprints/BP_SecondPhase.BP_SecondPhase_C|GetRootClicksCurrent _returnvalue_3) 1)))
      (Development|PrintString (Utilities|String|ToString(Integer) _output_get))
      (switch int (Variables|Default|GetWhereRootConnects)
        (:0
          ;[1 1 1] Activate children roots
          (Variables|Default|SetTotalRootsGrown (+ (Variables|Default|GetTotalRootsGrown) 1) :!label _label_2)
          (Variables|/Script/Engine.PlayerController|SetbEnableClickEvents _returnvalue true)
          (Variables|/Script/Engine.PlayerController|SetbEnableMouseOverEvents _returnvalue true))
        (:1
          (Utilities|FlowControl|Delay 3.0 :!label _label_3)
          (for _array_element (Variables|Default|GetRootChildren)
            (bind _asbp_root_grow_test (Utilities|Casting|CastToBP_RootGrowTest _array_element)
              (:then
                (Rendering|SetVisibility (Variables|BP_RootGrowTest_C|GetSK_Root02_WigglyAnim2 _asbp_root_grow_test) true false)
                (Variables|BP_RootGrowTest_C|SetIsClickable _asbp_root_grow_test true)
                (goto _label_2))
              (:CastFailed
                (goto _label_2)))))
        (:2
          (bind _returnvalue_4 (Actor|GetActorOfClass "/Game/EnvironmentAssets/ResourceIronTest.ResourceIronTest_C"))
          (Variables|/Game/EnvironmentAssets/ResourceIronTest.ResourceIronTest_C|SetCurrentIronNodesTouched _returnvalue_4 (+ (Variables|/Game/EnvironmentAssets/ResourceIronTest.ResourceIronTest_C|GetCurrentIronNodesTouched _returnvalue_4) 1))
          (switch int (Variables|Default|GetResourcesAndRootChildren) :!label _label_4
            (:0
              (Utilities|FlowControl|Delay 3.0 :!label _label_5)
              (goto _label_2))
            (:1
              (goto _label_3))))
        (:3
          (bind _returnvalue_5 (Actor|GetActorOfClass "/Game/EnvironmentAssets/ResourcePhosphorusTest.ResourcePhosphorusTest_C"))
          (Variables|/Game/EnvironmentAssets/ResourcePhosphorusTest.ResourcePhosphorusTest_C|SetCurrentPhosphorusNodesTouched _returnvalue_5 (+ (Variables|/Game/EnvironmentAssets/ResourcePhosphorusTest.ResourcePhosphorusTest_C|GetCurrentPhosphorusNodesTouched _returnvalue_5) 1))
          (goto _label_4))
        (:4
          (bind _returnvalue_6 (Actor|GetActorOfClass "/Game/EnvironmentAssets/ResourceNitrogenTest.ResourceNitrogenTest_C"))
          (Variables|/Game/EnvironmentAssets/ResourceNitrogenTest.ResourceNitrogenTest_C|SetCurrentNitrogenNodesTouched _returnvalue_6 (+ (Variables|/Game/EnvironmentAssets/ResourceNitrogenTest.ResourceNitrogenTest_C|GetCurrentNitrogenNodesTouched _returnvalue_6) 1))
          (goto _label_4))
        (:5
          (bind _returnvalue_7 (Actor|GetActorOfClass "/Game/EnvironmentAssets/ResourcePotassiumTest.ResourcePotassiumTest_C"))
          (Variables|/Game/EnvironmentAssets/ResourcePotassiumTest.ResourcePotassiumTest_C|SetCurrentPotassiumNodesTouched _returnvalue_7 (+ (Variables|/Game/EnvironmentAssets/ResourcePotassiumTest.ResourcePotassiumTest_C|GetCurrentPotassiumNodesTouched _returnvalue_7) 1))
          (goto _label_4))
        (:6
          (bind _returnvalue_8 (Actor|GetActorOfClass "/Game/EnvironmentAssets/ResourceZincTest.ResourceZincTest_C"))
          (Variables|/Game/EnvironmentAssets/ResourceZincTest.ResourceZincTest_C|SetCurrentZincNodesTouched _returnvalue_8 (+ (Variables|/Game/EnvironmentAssets/ResourceZincTest.ResourceZincTest_C|GetCurrentZincNodesTouched _returnvalue_8) 1))
          (goto _label_4)))
      (else
        ;[1 1 1] Make this into a text widget
        (Development|PrintString "You can No Longer Grow Roots!")
        (goto _label_5)))))

(event OnBeginCursorOver(Cube)
  (params (TouchedComponent :type Primitive%20Component%20Object%20Reference))
  (bind _sk_root02_wigglyanim2 (Variables|Default|GetSK_Root02_WigglyAnim2))
  ;[1 1 1] PREVIEW OUTLINE
  (if (Variables|Default|GetIsClickable)
    (Components|Animation|SetPosition _sk_root02_wigglyanim2 2e+01 true)
    (Rendering|Material|SetMaterial _sk_root02_wigglyanim2 0 "/Game/EnvironmentAssets/materials/MI_EMPTY.MI_EMPTY")
    (Rendering|Material|SetMaterial _sk_root02_wigglyanim2 1 "/Game/EnvironmentAssets/materials/MI_TreeRootsGHOST.MI_TreeRootsGHOST")
    (Rendering|SetVisibility _sk_root02_wigglyanim2 true false)))

(event OnEndCursorOver(Cube)
  (params (TouchedComponent :type Primitive%20Component%20Object%20Reference))
  (bind _sk_root02_wigglyanim2 (Variables|Default|GetSK_Root02_WigglyAnim2))
  ;[1 1 1] PREVIEW OUTLINE
  (if (Variables|Default|GetIsClickable)
    (Rendering|SetVisibility _sk_root02_wigglyanim2 false false)
    (Components|Animation|SetPosition _sk_root02_wigglyanim2 0.0 true)))

(event Custom|RootGrow)

(event EventBeginPlay
  (bind _sk_root02_wigglyanim2 (Variables|Default|GetSK_Root02_WigglyAnim2))
  (Utilities|FlowControl|DelayUntilNextTick)
  (for _array_element (Collision|GetOverlappingActors (Variables|Default|GetCollisionDetectionSphere) 0 :!class /Script/Engine.PrimitiveComponent)
    (if (Utilities|String|Contains (Utilities|GetDisplayName _array_element) "Iron")
      (Variables|Default|SetWhereRootConnects 2)
      (Development|PrintString "IRON DETECTED" true true "(R=1.000000,G=0.000000,B=0.160202,A=1.000000)" 2e+02)
      (else
        (Utilities|FlowControl|DelayUntilNextTick)
        (if (Utilities|String|Contains (Utilities|GetDisplayName _array_element) "Phosphorus")
          (Variables|Default|SetWhereRootConnects 3)
          (else
            (Utilities|FlowControl|DelayUntilNextTick)
            (if (Utilities|String|Contains (Utilities|GetDisplayName _array_element) "Nitrogen")
              (Variables|Default|SetWhereRootConnects 4)
              (else
                (Utilities|FlowControl|DelayUntilNextTick)
                (if (Utilities|String|Contains (Utilities|GetDisplayName _array_element) "Potassium")
                  (Variables|Default|SetWhereRootConnects 5)
                  (else
                    (Utilities|FlowControl|DelayUntilNextTick)
                    (if (Utilities|String|Contains (Utilities|GetDisplayName _array_element) "Zinc")
                      (Variables|Default|SetWhereRootConnects 6)))))))))))
  (Components|Animation|SetPosition _sk_root02_wigglyanim2 0.0 true)
  (Rendering|SetVisibility _sk_root02_wigglyanim2 (Variables|Default|GetIsClickable) false))

(fn ConstructionScript
  (bind _sk_root02_wigglyanim2 (Variables|Default|GetSK_Root02_WigglyAnim2))
  (bind _rootstylepicker (Variables|Default|GetRootStylePicker))
  (Variables|/Script/Engine.SceneComponent|SetbAbsoluteScale (Variables|Default|GetPlane) true)
  (Components|SkeletalMesh|SetSkeletalMeshAsset _sk_root02_wigglyanim2 (Utilities|Array|Get(acopy) (Variables|Default|GetRootStyle) _rootstylepicker))
  (switch int _rootstylepicker
    (:Default
      (Components|Animation|OverrideAnimationData _sk_root02_wigglyanim2 "/Game/EnvironmentAssets/models/SK_Root02_WigglyAnim2.SK_Root02_WigglyAnim2_Animation" false false 2e+01 1.0 :!label _label))
    (:0
      (goto _label))
    (:1
      (Components|Animation|OverrideAnimationData _sk_root02_wigglyanim2 "/Game/EnvironmentAssets/models/SK_Root03_ShortAnim.SK_Root03_ShortAnim_Animation" false false 2e+01 1.0))
    (:2
      (Components|Animation|OverrideAnimationData _sk_root02_wigglyanim2 "/Game/EnvironmentAssets/models/SK_Root04_LongAnim.SK_Root04_LongAnim_Animation" false false 2e+01 1.0))))
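; Background scenery actor of trees, bushes, grass and sky whose look shifts as waves progress.
; SetBackgroundColor takes the wave number and plays a timeline that advances the materials' CurveTime scalar through that wave's fraction of WaveTotal.
; The value goes to every static mesh component, so the materials handle the actual color change.
; Older per-wave color switches and a bird-plane slide animation remain unconnected, and the construction script does nothing.
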(event Custom|SetBackgroundColor
  (params (CurrentWaveNumber :type Integer))
  (Variables|Default|SetincrementSky (/ (- CurrentWaveNumber 1) (Variables|Default|GetWaveTotal)))
  (bind _animcurve (Timeline|Timeline PlayFromStart)
    (:Update
      (Rendering|Material|SetScalarParameterValueonMaterials (Actor|GetComponentsByClass "/Script/Engine.StaticMeshComponent") "CurveTime" (+ (Math|Float|SafeDivide _animcurve (Variables|Default|GetWaveTotal)) (Variables|Default|GetincrementSky))))))

(fn ConstructionScript)